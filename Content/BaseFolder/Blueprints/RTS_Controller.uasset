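; RTS player controller that pans and zooms the RTS_Cam view target, with the mouse locked in Game and UI input mode.
; WASD keys set X/Y step values and one shared pressed flag; both movement axis events apply those steps to camera location, unscaled by delta time.
; Mouse wheel changes spring arm length within clamped limits.
; Releasing any WASD key clears the shared flag, even if others remain held.
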(event `self.ReceiveBeginPlay`
  (`WidgetBlueprintLibrary.SetInputMode_GameAndUIEx` null null "LockAlways" false)
  (bind _asrts_cam (cast `/Game/BaseFolder/Blueprints/RTS_Cam` (`self.GetViewTarget`)))
  (set `self.RTSCam` _asrts_cam))

(event `Key|MouseScrollUp`
  (params (Key :type "Key Structure"))
  (bind _springarm (`/Game/BaseFolder/Blueprints/RTS_Cam.SpringArm` (`self.RTSCam`)))
  (:`Pressed`
    ;[1 1 1] Cam Zoom
    (set `SpringArmComponent.TargetArmLength` (`KismetMathLibrary.FClamp` (- (`SpringArmComponent.TargetArmLength` _springarm) 200.0) 1000.0 5000.0) _springarm)))

(event `Key|MouseScrollDown`
  (params (Key :type "Key Structure"))
  (bind _springarm (`/Game/BaseFolder/Blueprints/RTS_Cam.SpringArm` (`self.RTSCam`)))
  (:`Pressed`
    ;[1 1 1] Cam Zoom
    (set `SpringArmComponent.TargetArmLength` (`KismetMathLibrary.FClamp` (+ (`SpringArmComponent.TargetArmLength` _springarm) 200.0) 1000.0 5000.0) _springarm)))

(event `InputAxis|MoveForward`
  (params (AxisValue :type "Float (single-precision)"))
  (bind _rtscam (`self.RTSCam`))
  (bind (_returnvalue_x _returnvalue_y _returnvalue_z) (`KismetMathLibrary.BreakVector` (`self.K2_GetActorLocation` _rtscam)))
  (if (`self.W_Pressed`) :!label _label
    (`self.K2_SetActorRelativeLocation` _rtscam (`KismetMathLibrary.MakeVector` (+ _returnvalue_x (`KismetMathLibrary.Conv_IntToDouble` (`self.left-right`))) (+ _returnvalue_y (`KismetMathLibrary.Conv_IntToDouble` (`self.up-down`))) _returnvalue_z) false false)
    (else
      (`self.StopMovement` (`GameplayStatics.GetPlayerController` 0)))))

(event `InputAxis|MoveRight`
  (params (AxisValue :type "Float (single-precision)"))
  (goto _label))

(event `Key|W`
  (params (Key :type "Key Structure"))
  (:`Pressed`
    (set `self.W_Pressed` true)
    (set `self.up-down` (`self.speed`)))
  (:`Released`
    (set `self.W_Pressed` false)
    (set `self.up-down` 0)))

(event `Key|S`
  (params (Key :type "Key Structure"))
  (:`Pressed`
    (set `self.W_Pressed` true)
    (set `self.up-down` (* (`self.speed`) -1)))
  (:`Released`
    (set `self.W_Pressed` false)
    (set `self.up-down` 0)))

(event `Key|A`
  (params (Key :type "Key Structure"))
  (:`Pressed`
    (set `self.W_Pressed` true)
    (set `self.left-right` (`self.speed`)))
  (:`Released`
    (set `self.W_Pressed` false)
    (set `self.left-right` 0)))

(event `Key|D`
  (params (Key :type "Key Structure"))
  (:`Pressed`
    (set `self.W_Pressed` true)
    (set `self.left-right` (* (`self.speed`) -1)))
  (:`Released`
    (set `self.W_Pressed` false)
    (set `self.left-right` 0)))

(fn `UserConstructionScript`)