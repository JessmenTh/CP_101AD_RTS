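; RTS_GameMode is the game mode for an RTS game that serves as a global access point for the level's navigation volume and grid.
; On BeginPlay it finds the first NavMeshBoundsVolume and the first BP_Grid actor with GetAllActorsOfClass and caches them.
; GetNavMesh and GetGrid expose these cached references to other Blueprints.
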(event `self.ReceiveBeginPlay`
  (`|ExecutionSequence`
    (:`then_0`
      ;[1 1 1] make NaveMesh Global
      (bind _outactors (`GameplayStatics.GetAllActorsOfClass` "/Script/NavigationSystem.NavMeshBoundsVolume"))
      (set `self.NavMesh` (`|GetArrayItem` _outactors)))
    (:`then_1`
      ;[1 1 1] make Grid Global
      (bind _outactors_2 (`GameplayStatics.GetAllActorsOfClass` "/Game/BP_Grid.BP_Grid_C"))
      (set `self.Grid` (`|GetArrayItem` _outactors_2)))))

(fn `GetGrid`
  (returns (Grid :type "/Game/BP_Grid Object Reference"))
  (return (`self.Grid`)))

(fn `GetNavMesh`
  (returns (NavMesh :type "NavMeshBoundsVolume Object Reference"))
  (return (`self.NavMesh`)))

(fn `UserConstructionScript`)