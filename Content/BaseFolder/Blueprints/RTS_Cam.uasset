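; RTS camera actor that takes over player 0's view on BeginPlay and pans by screen-edge scrolling while Left Ctrl is held.
; Tick sets UseMouse from the key and, when true, calls four directional move functions.
; Each offsets the root component along X or Y, ramping speed across the outer 5% of the viewport using normalized, clamped mouse position.
; Movement is applied per frame, without delta-time scaling.
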(event `self.ReceiveBeginPlay`
  (`PlayerController.SetViewTargetWithBlend` (`GameplayStatics.GetPlayerController` 0) self 0.0 "VTBlend_Linear" 0.0 false))

(event `self.ReceiveTick`
  (params (DeltaSeconds :type "Float (single-precision)"))
  (bind _returnvalue (`GameplayStatics.GetPlayerController` 0))
  (`|ExecutionSequence`
    (:`then_0`
      ;[1 1 1] check for CamMovment via Mouse on or off
      (if (`PlayerController.WasInputKeyJustPressed` _returnvalue "LeftControl")
        (set `self.UseMouse` true)))
    (:`then_1`
      (if (`PlayerController.WasInputKeyJustReleased` _returnvalue "LeftControl")
        (set `self.UseMouse` false)))
    (:`then_2`
      ;[1 1 1] CamMovement
      (if (`self.UseMouse`)
        (`self.MoveLeft`)
        (`self.MoveRight`)
        (`self.MoveUp`)
        (`self.MoveDown`)))))

(fn `MoveDown`
  (bind (_returnvalue_x _returnvalue_y) (`KismetMathLibrary.BreakVector2D` (`WidgetLayoutLibrary.GetViewportSize`)))
  (bind _returnvalue (`WidgetLayoutLibrary.GetMousePositionOnViewport`))
  (`SceneComponent.K2_AddRelativeLocation` (`self.DefaultSceneRoot`) (* (0.0 -100.0 0.0) (`KismetMathLibrary.FClamp` (`KismetMathLibrary.NormalizeToRange` (* (`.Y` (`KismetMathLibrary.BreakVector2D` _returnvalue)) (`WidgetLayoutLibrary.GetViewportScale`)) (* _returnvalue_y 0.95) _returnvalue_y))) false false))

(fn `MoveLeft`
  (bind _returnvalue_x (`KismetMathLibrary.BreakVector2D` (`WidgetLayoutLibrary.GetViewportSize`)))
  (bind _returnvalue (`WidgetLayoutLibrary.GetMousePositionOnViewport`))
  (`SceneComponent.K2_AddRelativeLocation` (`self.DefaultSceneRoot`) (* (100.0 0.0 0.0) (- 1.0 (`KismetMathLibrary.FClamp` (`KismetMathLibrary.NormalizeToRange` (`KismetMathLibrary.BreakVector2D` _returnvalue) 0.0 (* (* _returnvalue_x (`WidgetLayoutLibrary.GetViewportScale`)) 0.05))))) false false))

(fn `MoveRight`
  (bind _returnvalue_x (`KismetMathLibrary.BreakVector2D` (`WidgetLayoutLibrary.GetViewportSize`)))
  (bind _returnvalue (`WidgetLayoutLibrary.GetMousePositionOnViewport`))
  (`SceneComponent.K2_AddRelativeLocation` (`self.DefaultSceneRoot`) (* (-100.0 0.0 0.0) (`KismetMathLibrary.FClamp` (`KismetMathLibrary.NormalizeToRange` (* (`KismetMathLibrary.BreakVector2D` _returnvalue) (`WidgetLayoutLibrary.GetViewportScale`)) (* _returnvalue_x 0.95) _returnvalue_x))) false false))

(fn `MoveUp`
  (bind (_returnvalue_x _returnvalue_y) (`KismetMathLibrary.BreakVector2D` (`WidgetLayoutLibrary.GetViewportSize`)))
  (bind _returnvalue (`WidgetLayoutLibrary.GetMousePositionOnViewport`))
  (`SceneComponent.K2_AddRelativeLocation` (`self.DefaultSceneRoot`) (* (0.0 100.0 0.0) (- 1.0 (`KismetMathLibrary.FClamp` (`KismetMathLibrary.NormalizeToRange` (`.Y` (`KismetMathLibrary.BreakVector2D` _returnvalue)) 0.0 (* (* _returnvalue_y (`WidgetLayoutLibrary.GetViewportScale`)) 0.05))))) false false))

(fn `UserConstructionScript`
  (set `self.UseMouse` false))